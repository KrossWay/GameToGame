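; BP_Player is the player Blueprint for a card game, handling the HUD and cursor interaction with cards.
; On BeginPlay it creates the main HUD widget and keeps a reference to it.
; Right click traces under the cursor and flips any BP_MasterCard it hits.
; Debug number keys push Russian test lines to the HUD text board, and an unconnected branch holds interface-based card destruction.
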(event `Key|One`
  (params (Key :type "Key Structure"))
  ;[1 1 1] debug SetText
  (:`Pressed`
    (`/Game/GameCore/Widgets/WBP_TextBoard.DialogText` (`/Game/GameCore/Widgets/WBP_MainHUD.WBP_TextBoard` (`self.MainWidgetRef`)) "Ну что народ")))

(event `Key|Two`
  (params (Key :type "Key Structure"))
  ;[1 1 1] debug SetText
  (:`Pressed`
    (`/Game/GameCore/Widgets/WBP_TextBoard.DialogText` (`/Game/GameCore/Widgets/WBP_MainHUD.WBP_TextBoard` (`self.MainWidgetRef`)) "Пора начинать!")))

(event `Key|Three`
  (params (Key :type "Key Structure"))
  ;[1 1 1] debug SetText
  (:`Pressed`
    (`/Game/GameCore/Widgets/WBP_TextBoard.DialogText` (`/Game/GameCore/Widgets/WBP_MainHUD.WBP_TextBoard` (`self.MainWidgetRef`)) (select `int` (`KismetMathLibrary.RandomInteger` 3) :`0` "А?" :`1` "А??" :`2` "А?!" :`3` "" :!type "Text"))))

(event `Key|Q`
  (params (Key :type "Key Structure"))
  ;[1 1 1] Debug destruct card
)

(event `InputAction|RightClick`
  (params (Key :type "Key Structure"))
  (bind (_hitresult _returnvalue) (`PlayerController.GetHitResultUnderCursorByChannel` (`GameplayStatics.GetPlayerController` 0) "TraceTypeQuery3" true))
  ;[1 1 1] Debug destruct card
  (:`Pressed`
    (if _returnvalue
      (bind _asbp_master_card (cast `/Game/GameCore/Blueprints/Card/BP_MasterCard` (`.HitActor` (`GameplayStatics.BreakHitResult` _hitresult))))
      (`/Game/GameCore/Blueprints/Card/BP_MasterCard.FlipFlopCard` _asbp_master_card))))

(event `self.ReceiveBeginPlay`
  (bind _returnvalue (`|CreateWidget` "/Game/GameCore/Widgets/WBP_MainHUD.WBP_MainHUD_C"))
  (bind _output_get (set `self.MainWidgetRef` _returnvalue))
  (`UserWidget.AddToViewport` _output_get 0))

(fn `UserConstructionScript`)