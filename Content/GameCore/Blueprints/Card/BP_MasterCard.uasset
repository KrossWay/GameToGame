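; Base card actor for a card game, with character, frame and backboard textures set through dynamic material instances.
; It slides up on a timeline, then allows two-stage MoveComponentTo flips; while face-up and hovered, a looping timer tilts it toward the cursor.
; Interaction on face-up cards goes to the GameMode, while placeholder logic branches on card type to show player lines through the HUD.
; Destruction applies radial damage to itself, then expires the actor.
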(event `SlideCardToTop`
  (params (Delay :type "Float (double-precision)") (Z :type "Float (double-precision)"))
  (bind (_startactorlocation_x _startactorlocation_y _startactorlocation_z) (`KismetMathLibrary.BreakVector` (`self.StartActorLocation`)))
  (set `self.StartActorLocation` (`self.K2_GetActorLocation`))
  (`KismetSystemLibrary.Delay` Delay)
  (bind (_direction _z) (`Timeline|ZOffset` :!via `PlayFromStart`)
    (:`Update`
      (`self.K2_SetActorLocation` (`KismetMathLibrary.VLerp` (`self.StartActorLocation`) (`KismetMathLibrary.MakeVector` _startactorlocation_x _startactorlocation_y (+ _startactorlocation_z Z)) _z)))
    (:`Finished`
      (set `self.SlideEnd` true))))

(event `self.ReceiveBeginPlay`
  (`MaterialInstanceDynamic.SetTextureParameterValue` (`self.CharacterTexture`) "CharacterTexture" (`self.IconCharacter2D`))
  (`MaterialInstanceDynamic.SetTextureParameterValue` (`self.FrameTexture`) "FrontCardFrame" (`self.IconFrame2D`))
  (`MaterialInstanceDynamic.SetTextureParameterValue` (`self.BackgroundTexture`) "BackgroundTexture" (`self.IconBackboard2D`)))

(event `FlipFlopCard`
  ;[1 0.7863 0.3424] FlipFlop Card
  (if (`self.SlideEnd`) :!label _label
    (`/Engine/EditorBlueprintResources/StandardMacros.DoOnce` false :!label _label_2
      (:`Completed`
        (bind _isa (`/Engine/EditorBlueprintResources/StandardMacros.FlipFlop`)
          (:`A`
            _)
          (:`B`
            _))
        (set `self.FaceToUp` _isa)
        (set `self.CanRotateToTarget` false)
        (set `self.StartPosition` (`self.K2_GetActorLocation`))
        (set `self.StartRotation` (`SceneComponent.K2_GetComponentRotation` (`self.Scene`)))
        (set `self.FlipPosition` (+ (`self.StartPosition`) (`KismetMathLibrary.MakeVector` 0.0 (`self.FlipHeightFromY`))))
        (`KismetSystemLibrary.MoveComponentTo` (`self.Scene`) (`self.FlipPosition`) (`KismetMathLibrary.ComposeRotators` (`self.StartRotation`) (struct :`Yaw` 90.0)) false true (`self.HalfTime`) true)
        (`KismetSystemLibrary.MoveComponentTo` (`self.Scene`) (`self.FlipPosition`) (`KismetMathLibrary.ComposeRotators` (`self.StartRotation`) (struct :`Yaw` 180.0)) true false (`self.HalfTime`) true)
        (set `self.CanRotateToTarget` true)
        (goto _label_2 :!via `Reset`)))))

(event `/Game/GameCore/Blueprints/Interfaces/BPI_InteractCard.FlipCard`
  ;[1 0.7863 0.3424] FlipFlop Card
  (goto _label))

(event `self.ReceiveActorBeginCursorOver`
  ;[1 1 1] Set card target to mouse cursor
  (bind _returnvalue (`KismetSystemLibrary.K2_SetTimer` null "LookForCursor" 0.01 true)))

(event `self.ReceiveActorEndCursorOver`
  ;[1 1 1] Set card target to mouse cursor
  (`KismetSystemLibrary.K2_ClearAndInvalidateTimerHandle` (stale `self.ReceiveActorBeginCursorOver` _returnvalue)))

(event `HeroAnswer`
  (params (HeroAnswer :type Text))
  ;[0 0.9382 1] DEBUG
)

(event `FAKE_WEAPON_TAKE`
  ;[0 0.9382 1] DEBUG
)

(event `/Game/GameCore/Blueprints/Interfaces/BPI_DamageInteract.DestroyCard`
  (`self.PlayDesctructable`))

(event `PlayDesctructable`
  ;[1 1 1] Interface for destroy mesh
  (if (`self.CanBeDestroy`)
    (`/Engine/EditorBlueprintResources/StandardMacros.DoOnce` false
      (:`Completed`
        (`GameplayStatics.ApplyRadialDamageWithFalloff` :`BaseDamage` 2.0 :`MinimumDamage` 2.0 :`Origin` (`self.K2_GetActorLocation`) :`DamageInnerRadius` 50.0 :`DamageOuterRadius` 100.0 :`DamageFalloff` 0.1 :`DamageCauser` null :`InstigatedByController` null)
        (`self.SetLifeSpan` 2.0)))))

(event `PlayerSay`
  (params (PlayerText :type Text))
  ;[0 0.9382 1] DEBUG
  (message `/Game/GameCore/Blueprints/Interfaces/BPI_GLOBAL_INTERACT.SHOW_CHARACTER_TEXT` (`PlayerController.GetHUD` (`GameplayStatics.GetPlayerController` 0)) PlayerText))

(event `Character`
  ;[0 0.9382 1] DEBUG
  ;;[1 1 1] если персонаж
  ;;[1 1 1] пишем текст который говорит игрок
  (`self.PlayerSay` (`self.PlayerTextToHero`)))

(event `/Game/GameCore/Blueprints/Interfaces/BPI_InteractCard.InteractWithCard`
  ;[1 1 1] Event Interact with card
  (if (`self.FaceToUp`)
    (message `/Game/GameCore/Blueprints/Interfaces/BPI_Player.StopInteract` (`GameplayStatics.GetPlayerPawn` 0))
    (message `/Game/GameCore/Blueprints/Interfaces/BPI_InteractCard.StartInteract` (`GameplayStatics.GetGameMode`) self)))

(event `FAKE_INTERACT`
  ;[0 0.9382 1] DEBUG
  ;;[1 1 1] INTERACT
  (switch `/Game/GameCore/Blueprints/Enums/E_CardType` (`self.CardType`)
    (:`NewEnumerator0`
      (`self.Character`))
    (:`NewEnumerator1`
      (`self.Weapon`))
    (:`NewEnumerator2`
      (`self.EventCardType`))))

(event `Weapon`
  ;[0 0.9382 1] DEBUG
  ;;[1 1 1] Если оружие
  ;;[1 1 1] Есть ли уже оружие в руке?
  (if (`self.HaveWeapon`)
    ;;[1 1 1] Говорим о том как нам жаль что мы не можем его взять
    (`self.PlayerSay` (`self.CannotTakeWeaponText`))
    (else
      ;;[1 1 1] Забираем оружие в ячейку
      (`self.FAKE_WEAPON_TAKE`)
      ;;[1 1 1] Игрок говорит как он рад находке
      (`self.PlayerSay` (`self.TakeWeaponText`))
      (set `self.HaveWeapon` true))))

(event `EventCardType`
  ;[0 0.9382 1] DEBUG
  (switch `/Game/GameCore/Blueprints/Enums/E_EventType` (`self.EventType`)
    (:`NewEnumerator0`)
    (:`NewEnumerator1`)
    (:`NewEnumerator2`
      ;;[1 1 1] Событие если, ничего не происходит влиятельного на сюжет
      (`self.PlayerSay` (`self.PlayerTextToEventNothing`)))))

(fn `LookForCursor`
  (bind _returnvalue (`GameplayStatics.GetWorldDeltaSeconds`))
  (bind (_returnvalue_roll _returnvalue_pitch _returnvalue_yaw) (`KismetMathLibrary.BreakRotator` (`self.K2_GetActorRotation`)))
  (bind (_returnvalue_roll_2 _returnvalue_pitch_2 _returnvalue_yaw_2) (`KismetMathLibrary.BreakRotator` (`KismetMathLibrary.FindLookAtRotation` (`self.K2_GetActorLocation`) (+ (`.Location` (`GameplayStatics.BreakHitResult` (`PlayerController.GetHitResultUnderCursorByChannel` (`GameplayStatics.GetPlayerController` 0) "TraceTypeQuery1" true))) (0.0 200.0 0.0)))))
  (if (and (`self.CanRotateToTarget`) (`self.FaceToUp`))
    (`self.K2_SetActorRotation` (`KismetMathLibrary.MakeRotator` _returnvalue_roll_2 (`KismetMathLibrary.FInterpTo` _returnvalue_pitch (`KismetMathLibrary.FClamp` _returnvalue_pitch_2 -10.0 10.0) _returnvalue 1.5) (`KismetMathLibrary.FInterpTo` _returnvalue_yaw (`KismetMathLibrary.FClamp` _returnvalue_yaw_2 80.0 110.0) _returnvalue 1.5)))))

(fn `UserConstructionScript`
  (bind _sm_card_dm (`self.SM_Card_DM`))
  (bind _returnvalue (`PrimitiveComponent.GetMaterial` _sm_card_dm 0))
  (bind _returnvalue_2 (`PrimitiveComponent.CreateDynamicMaterialInstance` _sm_card_dm 0 _returnvalue "None"))
  (set `self.CharacterTexture` _returnvalue_2)
  (bind _returnvalue_3 (`PrimitiveComponent.CreateDynamicMaterialInstance` _sm_card_dm 0 _returnvalue "None"))
  (set `self.FrameTexture` _returnvalue_3)
  (bind _returnvalue_4 (`PrimitiveComponent.CreateDynamicMaterialInstance` _sm_card_dm 0 _returnvalue "None"))
  (set `self.BackgroundTexture` _returnvalue_4))