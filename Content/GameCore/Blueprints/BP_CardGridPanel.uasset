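; BP_CardGridPanel is an actor that deals a shuffled set of card actors into a vertical grid when play begins.
; SpawnCards shuffles the card class list, then uses one entry per grid cell until rows and columns are filled or the list empties.
; Each card spawns rotated 180 degrees below the panel and receives SlideCardToTop with its X/Z cell target and a row- and column-based delay, staggering the deal.
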(event `self.ReceiveBeginPlay`
  (`self.SpawnCards` (`self.CardForSpawn`)))

(fn `SpawnCards`
  (params (TargetArray :type "Array of /Game/GameCore/Blueprints/Card/BP_MasterCard Class Reference (by ref)"))
  (locals (LocalCards :type "Array of /Game/GameCore/Blueprints/Card/BP_MasterCard Class Reference") (ZOffset :type "Float (double-precision)" :default -800.0))
  (bind (_returnvalue_x _returnvalue_y _returnvalue_z) (`KismetMathLibrary.BreakVector` (`self.K2_GetActorLocation`)))
  (bind _output_get (set `local.LocalCards` TargetArray))
  (`KismetArrayLibrary.Array_Shuffle` _output_get)
  (set `self.RootLocation` (`self.K2_GetActorLocation`))
  (for _index (range (`self.Row`))
    (for _index_2 (range (`self.Column`))
      (if (> (`KismetArrayLibrary.Array_Length` (`local.LocalCards`)) 0)
        (bind _returnvalue (`|SpawnActorFromClass` (`|GetArrayItem` (`local.LocalCards`)) (`KismetMathLibrary.MakeTransform` (`KismetMathLibrary.MakeVector` _returnvalue_x _returnvalue_y (- _returnvalue_z (`local.ZOffset`))) (`KismetMathLibrary.ComposeRotators` (`self.K2_GetActorRotation`) (struct :`Yaw` -180.0))) "Undefined" "OverrideRootScale" null null))
        (`/Game/GameCore/Blueprints/Card/BP_MasterCard.SlideCardToTop` _returnvalue (+ (* _index_2 0.5) (* (+ _index 1) 1.0)) (* (`local.ZOffset`) -1.0) (`KismetMathLibrary.MakeVector` (+ (.x (`self.RootLocation`)) (* _index_2 (`self.ColumnDistance`))) (.y (`self.RootLocation`)) (+ (.z (`self.RootLocation`)) (* _index (`self.RowDistance`)))))
        (`KismetArrayLibrary.Array_Remove` (`local.LocalCards`))))))

(fn `UserConstructionScript`)