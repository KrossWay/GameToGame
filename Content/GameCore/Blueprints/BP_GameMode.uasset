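; Game mode that mediates card dialog interactions between the BP_DirectorCards actor, found at BeginPlay, and the player HUD.
; StartInteract gets a card's type, dialog and answers from the director and sends them to the HUD.
; TakeAnswerIndex passes the chosen answer to the director, then destroys the card or restarts its interaction; taking it has no wired effect.
; A placeholder widget event shifts a story parameter toward happy or bad endings; CardClicked is debug-only.
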(event `self.ReceiveBeginPlay`
  (bind _outactors (`GameplayStatics.GetAllActorsOfClass` "/Game/GameCore/Blueprints/BP_DirectorCards.BP_DirectorCards_C"))
  (set `self.DirectorCardsRef` (`|GetArrayItem` _outactors))
  (`/Engine/EditorBlueprintResources/StandardMacros.IsValid` (`self.DirectorCardsRef`) :!label _label
    (:`Is Not Valid`
      (`KismetSystemLibrary.Delay` 0.2)
      (goto _label))))

(event `FAKE_WIDGET_EVENT`
  (params (QuestType :type "/Game/GameCore/Blueprints/Enums/E_QuestType Enum" :default "NewEnumerator0"))
  (bind _storyparametr (`self.StoryParametr`))
  ;[1 1 1] Отклоняемся от сюжета
  (switch `/Game/GameCore/Blueprints/Enums/E_QuestType` QuestType
    (:`NewEnumerator1`
      (`/Engine/EditorBlueprintResources/StandardMacros.IncrementInt` _storyparametr))
    (:`NewEnumerator2`
      (`/Engine/EditorBlueprintResources/StandardMacros.DecrementInt` _storyparametr))))

(event `Card Clicked`
  (params (interact_card :type "C_MasterCard Object Reference"))
  ;[1 1 1] DEBUG
  (bind (_card_type _dialog) (`C_ScriptDirector.ProcessDialog` (`self.DirectorCardsRef`) null))
  (switch `CardType` _card_type))

(event `/Game/GameCore/Blueprints/Interfaces/BPI_InteractCard.StartInteract`
  (params (CardRef :type "/Game/GameCore/Blueprints/Card/BP_MasterCard Object Reference"))
  ;[1 1 1] Start interact
  (bind _output_get (set `self.CurrentCardRef` CardRef))
  (bind (_card_type _dialog _answers) (`C_ScriptDirector.ProcessDialog` (`self.DirectorCardsRef`) _output_get))
  (message `/Game/GameCore/Blueprints/Interfaces/BPI_HUDinteract.ProcessInteract` (`PlayerController.GetHUD` (`GameplayStatics.GetPlayerController` 0)) _card_type _dialog _answers))

(event `/Game/GameCore/Blueprints/Interfaces/BPI_InteractCard.TakeAnswerIndex`
  (params (Index :type Integer))
  ;[1 1 1] Return answer player
  (bind (_dialog _action_with_card) (`C_ScriptDirector.ProcessDialogResult` (`self.DirectorCardsRef`) Index))
  (switch `ActionWithCard` _action_with_card
    (:`TAKE_CARD`
      (switch `EAppleTextureType` "Unknown" :!label _label_2))
    (:`KILL_CARD`
      (message `/Game/GameCore/Blueprints/Interfaces/BPI_DamageInteract.DestroyCard` (`self.CurrentCardRef`) 0.0)
      (goto _label_2))
    (:`BACK_CARD`
      (`/Game/GameCore/Blueprints/Interfaces/BPI_InteractCard.StartInteract` self (`self.CurrentCardRef`)))))

(fn `UserConstructionScript`)